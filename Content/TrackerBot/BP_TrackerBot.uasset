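; BP_TrackerBot is the Blueprint for a tracker bot, adding rolling-sound feedback based on its movement.
; Each tick it maps the bot's speed through a clamped range to the Audio component's volume multiplier, so faster rolling sounds louder.
; An unconnected debug snippet would find a navigation path to the player pawn and draw spheres at its points, but never runs.
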(event `self.ReceiveBeginPlay`)

(event `self.ReceiveTick`
  (params (DeltaSeconds :type "Float (single-precision)"))
  ;[1 1 1] Make rolling sound louder
  (`AudioComponent.SetVolumeMultiplier` (`self.Audio`) (`KismetMathLibrary.MapRangeClamped` (`KismetMathLibrary.VSize` (`self.GetVelocity`)) 10.0 1000.0 2.0 4.0)))

(fn `UserConstructionScript`)