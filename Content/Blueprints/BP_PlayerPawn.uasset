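; BP_PlayerPawn is the player pawn Blueprint, which currently handles only HUD setup.
; BeginPlay creates the crosshair and health indicator widgets and adds both to the viewport.
; The SHealth OnHealthChanged handler is empty.
; Disconnected nodes hold a disabled rifle spawn that attaches to the mesh's WeaponSocket, plus a health debug-text draw.
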(event `self.ReceiveBeginPlay`
  (`|ExecutionSequence`
    (:`then_0`
      (bind _returnvalue (`|CreateWidget` "/Game/UI/BP_Crosshair.BP_Crosshair_C"))
      (`UserWidget.AddToViewport` _returnvalue 0))
    (:`then_1`
      (bind _returnvalue_2 (`|CreateWidget` "/Game/UI/WBP_HealthIndicator.WBP_HealthIndicator_C"))
      (`UserWidget.AddToViewport` _returnvalue_2 0))))

(event `self.SHealth.OnHealthChanged`
  (params (HealthComp :type "SHealthComponent Object Reference") (Health :type "Float (single-precision)") (HealthDelta :type "Float (single-precision)") (DamageType :type "DamageType Object Reference") (InstigatedBy :type "Controller Object Reference") (DamageCauser :type "Actor Object Reference")))

(fn `UserConstructionScript`)